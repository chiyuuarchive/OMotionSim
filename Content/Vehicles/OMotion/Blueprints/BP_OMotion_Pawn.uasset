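; BP_OMotion_Pawn is the OMotion vehicle pawn, handling its removal, respawn and chassis material setup.
; Pressing Q calls RemoveFromScene to destroy the pawn, while Escape quits the game.
; On Destroyed, it asks BP_OMotionGameMode to respawn the player at the first BP_RespawnPoint found in the level.
; The construction script stores a dynamic instance of the mesh's first material as ChassisMaterial.
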(event `self.ReceiveDestroyed`
  (bind _outactors (`GameplayStatics.GetAllActorsOfClass` "/Game/Vehicles/OMotion/Blueprints/BP_RespawnPoint.BP_RespawnPoint_C"))
  (bind _asbp_omotion_game_mode (cast `/Game/Vehicles/OMotion/Blueprints/BP_OMotionGameMode` (`GameplayStatics.GetGameMode`)))
  (`/Game/Vehicles/OMotion/Blueprints/BP_OMotionGameMode.Respawn Player` _asbp_omotion_game_mode (`self.GetTransform` (`|GetArrayItem` _outactors))))

(event `Key|Q`
  (params (Key :type "Key Structure"))
  (:`Pressed`
    (`self.Remove From Scene`)))

(event `Remove From Scene`
  (`self.K2_DestroyActor`))

(event `Key|Escape`
  (params (Key :type "Key Structure"))
  (:`Pressed`
    (`KismetSystemLibrary.QuitGame` null "Quit")))

(fn `UserConstructionScript`
  (bind _returnvalue (`PrimitiveComponent.CreateDynamicMaterialInstance` (`self.Mesh`) 0 null "None"))
  (set `self.Chassis Material` _returnvalue))