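; Chaos vehicle pawn for OMotion that exposes scripted throttle and brake test events, resetting to its start transform with player input disabled.
; On destruction, it asks the game mode to respawn the player at the first BP_RespawnPoint.
; Helper functions measure acceleration and stopping time, distance and wheel rotations, but their tick and space-bar triggers are disconnected.
; The rotation counter reads wheel 0 for every index.
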(event `Key|SpaceBar`
  (params (Key :type "Key Structure")))

(event `self.ReceiveTick`
  (params (DeltaSeconds :type "Float (single-precision)")))

(event `self.ReceiveBeginPlay`
  ;[1 1 1] Set respawn location
  (set `self.startingTransform` (`self.GetTransform`)))

(event `RemoveVehicle`
  ;[1 1 1] When vehicle is destroyed, spawn at test location
  (`self.K2_DestroyActor`))

(event `self.ReceiveDestroyed`
  ;[1 1 1] When vehicle is destroyed, spawn at test location
  (bind _outactors (`GameplayStatics.GetAllActorsOfClass` "/Game/OMotion/Blueprints/BP_RespawnPoint.BP_RespawnPoint_C"))
  (bind _asbp_omotion_game_mode (cast `/Game/OMotion/Blueprints/BP_OMotionGameMode` (`GameplayStatics.GetGameMode`)))
  (`/Game/OMotion/Blueprints/BP_OMotionGameMode.Respawn Player` _asbp_omotion_game_mode (`self.GetTransform` (`|GetArrayItem` _outactors))))

(event `StartThrottleTest`
  ;[1 1 1] Vehicle throttle events
  (`ChaosVehicleMovementComponent.ResetVehicle` (`self.VehicleMovementComponent`))
  (`self.K2_SetActorTransform` (`self.startingTransform`) false true)
  (`self.DisableInput` (`GameplayStatics.GetPlayerController` 0))
  (`KismetSystemLibrary.Delay` 1.0)
  (`ChaosVehicleMovementComponent.SetThrottleInput` (`self.VehicleMovementComponent`) 1.0))

(event `StopThrottle`
  ;[1 1 1] Vehicle throttle events
  (`ChaosVehicleMovementComponent.SetThrottleInput` (`self.VehicleMovementComponent`) 0.0))

(event `EndThrottleTest`
  ;[1 1 1] Vehicle throttle events
  (`self.EnableInput` (`GameplayStatics.GetPlayerController` 0)))

(event `StartBraking`
  ;[1 1 1] Vehicle brake events
  (`self.StopThrottle`)
  (`ChaosVehicleMovementComponent.SetBrakeInput` (`self.VehicleMovementComponent`) 1.0))

(event `StopBraking`
  ;[1 1 1] Vehicle brake events
  (`ChaosVehicleMovementComponent.SetBrakeInput` (`self.VehicleMovementComponent`) 0.0))

(fn `CalculateWheelRotation`
  (params (wheelIndex :type Integer))
  (bind _output (`|GetArrayItem` (`self.WheelAngles`) wheelIndex))
  (if (and (`self.IsCarMoving`) (`self.measureWheelRotation`))
    (bind _aschaos_wheeled_vehicle_movement_component (cast `ChaosWheeledVehicleMovementComponent` (`self.VehicleMovementComponent`)))
    (bind _returnvalue (`ChaosVehicleWheel.GetRotationAngle` (`|GetArrayItem` (`ChaosWheeledVehicleMovementComponent.Wheels` _aschaos_wheeled_vehicle_movement_component))))
    (if (< _output _returnvalue)
      (`|VariableSetRef` _output _returnvalue)
      (`/Engine/EditorBlueprintResources/StandardMacros.IncrementInt` (`|GetArrayItem` (`self.fulWheelRotations`) wheelIndex))
      (else
        (`|VariableSetRef` _output _returnvalue)))))

(fn `CheckStopped`
  (locals (DecelerationString :type String) (StopStimeString :type String) (DistanceString :type String) (wheelRotationString :type String))
  (bind _fulwheelrotations (`self.fulWheelRotations`))
  (bind _deccelerationrotations (`self.DeccelerationRotations`))
  (bind _timer (`self.timer`))
  (bind _returnvalue (/ (`self.targetSpeed`) (`self.timer`)))
  (bind _returnvalue_2 (* (`KismetMathLibrary.Vector_Distance` (`self.startingPosition`) (`SceneComponent.K2_GetComponentLocation` (`self.Mesh`))) 0.01))
  (if (and (`self.timerTicking`) (`self.targetSpeedReached`))
    (if (<= (* (`ChaosVehicleMovementComponent.GetForwardSpeed` (`self.VehicleMovementComponent`)) 0.036) 0.0)
      (`self.StopTimer`)
      (bind _output_get (set `local.DecelerationString` "Decceleration: "))
      (`KismetSystemLibrary.PrintString` (`KismetStringLibrary.Concat_StrStr` _output_get (`KismetStringLibrary.Conv_DoubleToString` _returnvalue)))
      (set `self.Decceleration` _returnvalue)
      (bind _output_get_2 (set `local.StopStimeString` "Time to stop: "))
      (`KismetSystemLibrary.PrintString` (`KismetStringLibrary.Concat_StrStr` _output_get_2 (`KismetStringLibrary.Conv_DoubleToString` _timer)))
      (set `self.DeccelerationTime` _timer)
      (bind _output_get_3 (set `local.DistanceString` "Distance: "))
      (`KismetSystemLibrary.PrintString` (`KismetStringLibrary.Concat_StrStr` _output_get_3 (`KismetStringLibrary.Conv_DoubleToString` _returnvalue_2)))
      (set `self.DeccelerationDistance` _returnvalue_2)
      (`|VariableSetRef` (`|GetArrayItem` _deccelerationrotations) (`|GetArrayItem` _fulwheelrotations))
      (`|VariableSetRef` (`|GetArrayItem` _deccelerationrotations 1) (`|GetArrayItem` _fulwheelrotations 1))
      (`|VariableSetRef` (`|GetArrayItem` _deccelerationrotations 2) (`|GetArrayItem` _fulwheelrotations 2)))))

(fn `CheckTargetSpeed`
  (locals (accelTimeString :type String) (totalTimeString :type String) (distanceString :type String) (wheelRotationsString :type String))
  (bind _fulwheelrotations (`self.fulWheelRotations`))
  (bind _accelrotations (`self.AccelRotations`))
  (bind _timer (`self.timer`))
  (bind _returnvalue (`SceneComponent.K2_GetComponentLocation` (`self.Mesh`)))
  (bind _output (`|GetArrayItem` _fulwheelrotations))
  (bind _output_2 (`|GetArrayItem` _fulwheelrotations 1))
  (bind _output_3 (`|GetArrayItem` _fulwheelrotations 2))
  (bind _returnvalue_2 (/ (* (`ChaosVehicleMovementComponent.GetForwardSpeed` (`self.VehicleMovementComponent`)) 0.036) (`self.timer`)))
  (bind _returnvalue_3 (* (`KismetMathLibrary.Vector_Distance` (`self.startingPosition`) _returnvalue) 0.01))
  (if (and (`self.timerTicking`) (not (`self.targetSpeedReached`)))
    (if (>= (* (`ChaosVehicleMovementComponent.GetForwardSpeed` (`self.VehicleMovementComponent`)) 0.036) (`self.targetSpeed`))
      (`self.StopTimer`)
      (set `self.targetSpeedReached` true)
      (bind _output_get (set `local.accelTimeString` "Acceleration: "))
      (`KismetSystemLibrary.PrintString` (`KismetStringLibrary.Concat_StrStr` _output_get (`KismetStringLibrary.Conv_DoubleToString` _returnvalue_2)))
      (set `self.Acceleration` _returnvalue_2)
      (bind _output_get_2 (set `local.totalTimeString` "TimeToReachSpeed: "))
      (`KismetSystemLibrary.PrintString` (`KismetStringLibrary.Concat_StrStr` _output_get_2 (`KismetStringLibrary.Conv_DoubleToString` _timer)))
      (set `self.AccelerationTime` _timer)
      (bind _output_get_3 (set `local.distanceString` "Distance: "))
      (`KismetSystemLibrary.PrintString` (`KismetStringLibrary.Concat_StrStr` _output_get_3 (`KismetStringLibrary.Conv_DoubleToString` _returnvalue_3)))
      (set `self.AccelerationDistance` _returnvalue_3)
      (set `self.startingPosition` _returnvalue)
      (set `local.wheelRotationsString` "WheelRotations: ")
      (`KismetSystemLibrary.PrintString` "Hello")
      ;[1 1 1] Save Values
      (`|VariableSetRef` (`|GetArrayItem` _accelrotations) _output)
      (`|VariableSetRef` (`|GetArrayItem` _accelrotations 1) _output_2)
      (`|VariableSetRef` (`|GetArrayItem` _accelrotations 2) _output_3)
      ;[1 1 1] Reset Measurements
      (`|VariableSetRef` _output)
      (`|VariableSetRef` _output_2)
      (`|VariableSetRef` _output_3)
      (set `self.timer` 0.0)
      (`ChaosVehicleMovementComponent.SetThrottleInput` (`self.VehicleMovementComponent`) 0.0)
      (`self.ResetTimer`)
      (`self.StartTimer`))))

(fn `IsCarMoving`
  (returns (output :type Boolean))
  (bind _returnvalue (`ChaosVehicleMovementComponent.GetForwardSpeed` (`self.VehicleMovementComponent`)))
  (return (or (> _returnvalue 1.0) (< _returnvalue -1.0))))

(fn `ResetTimer`
  (set `self.timerTicking` false)
  (set `self.timer` 0.0))

(fn `StartTimer`
  (set `self.timerTicking` true))

(fn `StopTimer`
  (set `self.timerTicking` false))

(fn `TickTimer`
  (params (deltaTime :type "Float (double-precision)"))
  (if (`self.timerTicking`)
    (set `self.timer` (+ (`self.timer`) deltaTime))))

(fn `UserConstructionScript`
  (bind _returnvalue (`PrimitiveComponent.CreateDynamicMaterialInstance` (`self.Mesh`) 0 null "None"))
  (set `self.Chassis Material` _returnvalue))